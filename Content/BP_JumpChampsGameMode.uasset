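; Game mode for Jump Champs that spawns players on login and periodically drops random weapons into the level.
; Tick runs through a five-second Delay, then picks a random WeaponsDataList row and calls SpawnWeapon with its stats and sprites at a random Y/Z position on the X=0 plane.
; PostLogin spawns a BP_PlayerCharacterController at the PlayerStart indexed by player count and has the new player possess it.
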(event `self.ReceiveBeginPlay`)

(event `self.ReceiveTick`
  (params (DeltaSeconds :type "Float (single-precision)"))
  (`KismetSystemLibrary.Delay` 5.0)
  (bind _outrownames (`DataTableFunctionLibrary.GetDataTableRowNames` "/Game/WeaponsDataList.WeaponsDataList"))
  (bind _returnvalue (`|GetDataTableRow` "/Game/WeaponsDataList.WeaponsDataList" (`|GetArrayItem` _outrownames (`KismetMathLibrary.RandomInteger` (`KismetArrayLibrary.Array_Length` _outrownames))))
    (:`then`
      (bind (_name _stackcapacity _bulletspeed _damage _firerate _weaponsprite _bulletsprite) (break `/Game/WeaponData` _returnvalue))
      (`self.spawnWeapon` (`KismetMathLibrary.MakeTransform` (`KismetMathLibrary.MakeVector` 0.0 (`KismetMathLibrary.RandomFloatInRange` 2000.0) (`KismetMathLibrary.RandomFloatInRange` 100.0 300.0)) (struct :`Yaw` 90.0)) _stackcapacity _firerate _damage _bulletspeed _bulletsprite _weaponsprite)
      (`KismetSystemLibrary.PrintString` "Spawn"))))

(event `self.K2_PostLogin`
  (params (NewPlayer :type "PlayerController Object Reference"))
  (bind _outactors (`GameplayStatics.GetAllActorsOfClass` "/Script/Engine.PlayerStart"))
  (`|SpawnActorFromClass` "/Game/Character/BP_PlayerCharacterController.BP_PlayerCharacterController_C" (`self.GetTransform` (`|GetArrayItem` _outactors (- (`KismetArrayLibrary.Array_Length` (`GameStateBase.PlayerArray` (`GameplayStatics.GetGameState`))) 1))) "AlwaysSpawn" "OverrideRootScale" null null)
  (`Controller.Possess` NewPlayer null))

(fn `UserConstructionScript`)