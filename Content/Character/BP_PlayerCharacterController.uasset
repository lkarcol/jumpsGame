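; Player controller for BP_MainCharacter that handles sideways movement and mouse-aimed weapon fire.
; The Right axis calls PerformMove, which adds movement input along the pawn's right vector.
; Fire sends mouse and projected pawn screen positions to ServerFire, which maps their difference onto the world Y-Z plane for aim rotation.
; It then calls Shot on the active weapon, spawning an automatically replicated projectile on the server.
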(event `InputAxis|Right`
  (params (AxisValue :type "Float (single-precision)"))
  (`self.PerformMove` AxisValue))

(event `InputAction|Fire`
  (params (Key :type "Key Structure"))
  (bind (_locationx _locationy) (`self.GetMousePosition`))
  (:`Pressed`
    (`self.ServerFire` (`KismetMathLibrary.MakeVector2D` _locationx _locationy) (`self.ProjectWorldLocationToScreen` (`self.K2_GetActorLocation` (`self.K2_GetPawn`))))))

(event `ServerFire`
  (params (MouseLocation :type "Vector2D Structure") (ScreenLocation :type "Vector2D Structure"))
  (bind _returnvalue (`self.K2_GetPawn`))
  (bind (_x _y) (`KismetMathLibrary.BreakVector2D` ScreenLocation))
  (bind (_x_2 _y_2) (`KismetMathLibrary.BreakVector2D` MouseLocation))
  (bind _returnvalue_2 (`self.K2_GetActorLocation` _returnvalue))
  ;[0.272 1 0.7669] Na servery spawne projektice actor , ktory je uz automaticky replikovany vsetkym
  (bind _asbp_main_character (cast `/Game/Character/BP_MainCharacter` _returnvalue))
  (bind _returnvalue_3 (`MainPaperCharacter.getActiveWeapon` _asbp_main_character))
  (`/Engine/EditorBlueprintResources/StandardMacros.IsValid` _returnvalue_3
    (:`Is Valid`
      (`Weapon.shot` _returnvalue_3 (`KismetMathLibrary.MakeTransform` _returnvalue_2 (`KismetMathLibrary.MakeRotator` 0.0 (.pitch (`KismetMathLibrary.FindLookAtRotation` _returnvalue_2 (`KismetMathLibrary.MakeVector` (.x _returnvalue_2) (+ (.y _returnvalue_2) (- _x _x_2)) (+ (.z _returnvalue_2) (- _y _y_2))))) (.yaw (`KismetMathLibrary.FindLookAtRotation` _returnvalue_2 (`KismetMathLibrary.MakeVector` (.x _returnvalue_2) (+ (.y _returnvalue_2) (- _x _x_2)) (+ (.z _returnvalue_2) (- _y _y_2)))))))))))

(fn `PerformMove`
  (params (MoveRight :type "Float (double-precision)"))
  (bind _returnvalue (`self.K2_GetPawn`))
  (bind _asbp_main_character (cast `/Game/Character/BP_MainCharacter` _returnvalue))
  (`Pawn.AddMovementInput` _asbp_main_character (`self.GetActorRightVector` _returnvalue) MoveRight false))

(fn `UserConstructionScript`)